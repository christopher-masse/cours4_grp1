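; BP_Platform is a platform actor that rises vertically from its starting position when told to move.
; It stores the root's world location on BeginPlay, then StartMoving plays a Timeline whose alpha lerps the height offset from zero to LiftHeight.
; StopMoving stops the Timeline in place, so a later StartMoving resumes from that point.
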(event `self.ReceiveBeginPlay`
  (set `self.Start Location` (`SceneComponent.K2_GetComponentLocation` (`self.DefaultSceneRoot`))))

(event `Start Moving`
  (bind (_start_location_x _start_location_y _start_location_z) (`KismetMathLibrary.BreakVector` (`self.Start Location`)))
  (bind (_direction _alpha) (`Timeline|Timeline` :!label _label)
    (:`Update`
      (`SceneComponent.K2_SetWorldLocationAndRotation` :`self` (`self.DefaultSceneRoot`) :`NewLocation` (`KismetMathLibrary.MakeVector` _start_location_x _start_location_y (+ _start_location_z (`KismetMathLibrary.Lerp` 0.0 (`self.Lift Height`) _alpha)))))))

(event `Stop Moving`
  (goto _label :!via `Stop`))

(fn `StartMoving`
  (`self.StartMoving`))

(fn `StopMoving`
  (`self.StopMoving`))

(fn `UserConstructionScript`)